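; BP_Door_Exam is a door that opens onto the Lvl_Esame level once the game mode's button counter equals two.
; DoorOpen checks ButtonCounter on BP_ThirdPersonGameMode, then loads Lvl_Esame as a level instance and hides the door with its collision disabled.
; DoorClose restores visibility and collision without unloading the level; neither event is called within this Blueprint.
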(event `DoorOpen`
  (bind _asbp_third_person_game_mode (cast `/Game/ThirdPerson/Blueprints/BP_ThirdPersonGameMode` (`GameplayStatics.GetGameMode`)))
  (if (== (`/Game/ThirdPerson/Blueprints/BP_ThirdPersonGameMode.ButtonCounter` _asbp_third_person_game_mode) 2)
    (`LevelStreamingDynamic.LoadLevelInstanceBySoftObjectPtr` "/Game/Esame/Levels/Lvl_Esame.Lvl_Esame" (0.0 0.0 0.0) (struct) "" null)
    (`SceneComponent.SetVisibility` (`self.Door`) false false)
    (`PrimitiveComponent.SetCollisionEnabled` (`self.Door`) "NoCollision")))

(event `DoorClose`
  (`SceneComponent.SetVisibility` (`self.Door`) true false)
  (`PrimitiveComponent.SetCollisionEnabled` (`self.Door`) "QueryAndPhysics"))

(fn `UserConstructionScript`)